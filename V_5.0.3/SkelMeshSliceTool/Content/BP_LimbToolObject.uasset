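; BP_LimbToolObject is a tree node for a limb tool, holding bone data, child nodes and an assigned widget.
; SetVisibilityOnChildObjects recurses through SetVisOnChildren to collapse descendant widgets when Condition is true, skipping root-flagged nodes, or show them when false.
; CheckForDuplicateBoneName removes children sharing this node's bone, modifying the array while iterating it.
; PrintStats prints the node's and its children's bone names for debugging.
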(event `CheckForDuplicateBoneName`
  (bind _childobjects (`self.ChildObjects`))
  (bind _bonedata_bone (break `BoneHierachyStruct` (`self.BoneData`)))
  (for _array_element _childobjects
    (bind _asbp_limb_tool_object (cast `/Game/BP_LimbToolObject` _array_element))
    (bind _bonedata_bone_2 (break `BoneHierachyStruct` (`/Game/BP_LimbToolObject.BoneData` _asbp_limb_tool_object)))
    (if (== _bonedata_bone_2 _bonedata_bone)
      (`KismetArrayLibrary.Array_RemoveItem` _childobjects _array_element))))

(event `PrintStats`
  (bind _bonedata_bone (break `BoneHierachyStruct` (`self.BoneData`)))
  (`KismetSystemLibrary.PrintString` self (`KismetStringLibrary.Conv_NameToString` _bonedata_bone))
  (for _array_element (`self.ChildObjects`)
    (bind _asbp_limb_tool_object (cast `/Game/BP_LimbToolObject` _array_element))
    (bind _bonedata_bone_2 (break `BoneHierachyStruct` (`/Game/BP_LimbToolObject.BoneData` _asbp_limb_tool_object)))
    (`KismetSystemLibrary.PrintString` self (`KismetStringLibrary.Concat_StrStr` "     " (`KismetStringLibrary.Conv_NameToString` _bonedata_bone_2)))))

(event `SetVisibilityOnChildObjects`
  (params (Condition :type Boolean))
  ;[1 1 1] Collapse or set VIsible the ChildObject array objects
  (`self.SetVisOnChildren` Condition))

(fn `SetVisOnChildren`
  (params (Condition :type Boolean))
  (if (> (`KismetArrayLibrary.Array_Length` (`self.ChildObjects`)) 0)
    (if (`local.Condition`)
      (for _array_element (`self.ChildObjects`)
        (`/Engine/EditorBlueprintResources/StandardMacros.IsValid` _array_element
          (:`Is Valid`
            (bind _asbp_limb_tool_object (cast `/Game/BP_LimbToolObject` _array_element))
            (if (`/Game/BP_LimbToolObject.IsRoot` _asbp_limb_tool_object)
              (bind _assignedwidget (`/Game/BP_LimbToolObject.AssignedWidget` _asbp_limb_tool_object))
              (`KismetSystemLibrary.PrintString` _assignedwidget (`KismetStringLibrary.Concat_StrStr` "IsRoot - " (`KismetSystemLibrary.GetDisplayName` _asbp_limb_tool_object)))
              (else
                (`Widget.SetVisibility` _assignedwidget "Collapsed")))
            (`self.SetVisibilityOnChildObjects` _asbp_limb_tool_object (`local.Condition`)))))
      (else
        (for _array_element_2 (`self.ChildObjects`)
          (`/Engine/EditorBlueprintResources/StandardMacros.IsValid` _array_element_2
            (:`Is Valid`
              (bind _asbp_limb_tool_object_2 (cast `/Game/BP_LimbToolObject` _array_element_2))
              (`Widget.SetVisibility` (`/Game/BP_LimbToolObject.AssignedWidget` _asbp_limb_tool_object_2) "Visible")
              (`self.SetVisibilityOnChildObjects` _asbp_limb_tool_object_2 (`local.Condition`)))))))))